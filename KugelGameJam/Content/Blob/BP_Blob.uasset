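; A collectible blob that awards PunkteBlob points to the PhysicsBallBP that overlaps its sphere.
; A quarter second after overlap, it hides, disables collision and adds to the ball's Score.
; Tick then restores visibility and collision through a random 10–20 second Delay, which keeps cycling because the Destroy flag is never cleared.
; The construction script applies the Material variable to the mesh.
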(event OnComponentBeginOverlap(Sphere)
  (params (OtherActor :type Actor%20Object%20Reference) (OtherComp :type Primitive%20Component%20Object%20Reference) (OtherBodyIndex :type Integer) (bFromSweep :type Boolean) (SweepResult :type Hit%20Result%20Structure%20%28by%20ref%29))
  (Utilities|FlowControl|Delay 0.25)
  (bind _asphysics_ball_bp (Utilities|Casting|CastToPhysicsBallBP OtherActor))
  (Rendering|SetVisibility (Variables|Default|GetSphere) false false)
  (Collision|SetCollisionEnabled (Variables|Default|GetStaticMesh) "NoCollision")
  (Variables|Default|SetDestroy true)
  (Variables|/Game/RollingBP/Blueprints/PhysicsBallBP.PhysicsBallBP_C|SetScore _asphysics_ball_bp (+ (Variables|/Game/RollingBP/Blueprints/PhysicsBallBP.PhysicsBallBP_C|GetScore _asphysics_ball_bp) (Variables|Default|GetPunkteBlob))))

(event EventTick
  (params (DeltaSeconds :type Float%20%28single-precision%29))
  (if (Variables|Default|GetDestroy)
    (Utilities|FlowControl|Delay (Math|Random|RandomFloatinRange 1e+01 2e+01))
    (Rendering|SetVisibility (Variables|Default|GetSphere) true false)
    (Collision|SetCollisionEnabled (Variables|Default|GetStaticMesh) "QueryAndPhysics")))

(event EventBeginPlay
  (Variables|Default|SetCurrentMaterial (Utilities|Array|Get(acopy) (Rendering|Material|GetMaterials (Variables|Default|GetStaticMesh)))))

(fn ConstructionScript
  (Rendering|Material|SetMaterial (Variables|Default|GetStaticMesh) 0 (Variables|Default|GetMaterial)))