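; A door Blueprint that opens only for a PhysicsBallBP whose material matches its DoorMaterial, which the construction script applies to the mesh.
; On a matching box overlap it adds Punkte to the ball's Score, hides the mesh and box, disables their collision and sets Open.
; While Open, Tick runs a random Delay to restore visibility and collision; Open is never reset, so this restore keeps repeating.
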(event OnComponentBeginOverlap(Box)
  (params (OtherActor :type Actor%20Object%20Reference) (OtherComp :type Primitive%20Component%20Object%20Reference) (OtherBodyIndex :type Integer) (bFromSweep :type Boolean) (SweepResult :type Hit%20Result%20Structure%20%28by%20ref%29))
  (bind _asphysics_ball_bp (Utilities|Casting|CastToPhysicsBallBP OtherActor))
  (bind _output_get (Variables|Default|SetBallMaterial (Rendering|Material|GetMaterial (Variables|/Game/RollingBP/Blueprints/PhysicsBallBP.PhysicsBallBP_C|GetBall _asphysics_ball_bp) 0)))
  (if (== _output_get (Variables|Default|GetDoorMaterial))
    (Variables|/Game/RollingBP/Blueprints/PhysicsBallBP.PhysicsBallBP_C|SetScore _asphysics_ball_bp (+ (Variables|/Game/RollingBP/Blueprints/PhysicsBallBP.PhysicsBallBP_C|GetScore _asphysics_ball_bp) (Variables|Default|GetPunkte)))
    (Rendering|SetVisibility (Variables|Default|GetStaticMesh) false false)
    (Collision|SetCollisionEnabled (Variables|Default|GetBox) "NoCollision")
    (Variables|Default|SetOpen true)))

(event EventTick
  (params (DeltaSeconds :type Float%20%28single-precision%29))
  (if (Variables|Default|GetOpen)
    (Utilities|FlowControl|Delay (Math|Random|RandomFloatinRange 2e+01 35.0))
    (Rendering|SetVisibility (Variables|Default|GetStaticMesh) true false)
    (Collision|SetCollisionEnabled (Variables|Default|GetBox) "QueryAndPhysics")))

(event EventBeginPlay)

(event EventActorBeginOverlap
  (params (OtherActor :type Actor%20Object%20Reference)))

(event EventTick
  (params (DeltaSeconds :type Float%20%28single-precision%29)))

(fn ConstructionScript
  (Rendering|Material|SetMaterial (Variables|Default|GetStaticMesh) 0 (Variables|Default|GetDoorMaterial)))